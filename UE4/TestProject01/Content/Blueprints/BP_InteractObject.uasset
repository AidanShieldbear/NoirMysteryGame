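; BP_InteractObject is an interactable object, such as a door or drawer, that toggles between open and closed.
; InteractWIthObject flips the Closed flag and plays or reverses a timeline, with Move choosing sliding or rotation.
; The timeline blend scales the X, Y and Z variables into the mesh's relative location or rotation.
; The construction script applies a uniform MeshScale and an optional mesh override.
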(event `InteractWIthObject`
  (if (`self.Move?`)
    (if (`self.Closed?`)
      (set `self.Closed?` false)
      (bind (_direction _blend) (`Timeline|BlendOpenClose` :!label _label)
        (:`Update`
          (`SceneComponent.K2_SetRelativeLocation` (`self.DefaultMesh`) (`KismetMathLibrary.MakeVector` (* _blend (`self.X`)) (* _blend (`self.Y`)) (* _blend (`self.Z`))) false false)))
      (else
        (set `self.Closed?` true)
        (goto _label :!via `Reverse`)))
    (elif (`self.Closed?`)
      (set `self.Closed?` false)
      (bind (_direction_2 _blend_2) (`Timeline|BlendRotate` :!via `PlayFromStart` :!label _label_2)
        (:`Update`
          (`SceneComponent.K2_SetRelativeRotation` (`self.DefaultMesh`) (`KismetMathLibrary.MakeRotator` (* _blend_2 (`self.X`)) (* _blend_2 (`self.Y`)) (* _blend_2 (`self.Z`))) false false)))
      (else
        (set `self.Closed?` true)
        (goto _label_2 :!via `ReverseFromEnd`)))))

(fn `UserConstructionScript`
  (bind _mesh_scale (`self.Mesh Scale`))
  (bind _objectmesh (`self.ObjectMesh`))
  ;[1 1 1] Set Mesh Scale
  (`SceneComponent.SetRelativeScale3D` (`self.DefaultMesh`) (`KismetMathLibrary.MakeVector` _mesh_scale _mesh_scale _mesh_scale))
  ;[1 1 1] Allow Mesh Override
  (if (!= _objectmesh null)
    (`StaticMeshComponent.SetStaticMesh` (`self.DefaultMesh`) _objectmesh)))